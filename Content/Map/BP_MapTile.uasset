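; Procedural map tile that grows a bathroom-themed level by spawning the next BP_MapTile from itself.
; Once the game mode accepts it, it opens a random gate and chains a tile there, counting TilesLeft down until it places a toilet portal instead.
; OpenGate opens the gate nearest another given tile.
; Prop sprites are randomized at construction; enemy spawns and the shower's presence at BeginPlay.
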(event EventBeginPlay
  (bind _asbp_game_mode (Utilities|Casting|CastToBP_GameMode (Game|GetGameMode)))
  (bind _ok (Default|AddTile _asbp_game_mode self))
  (if _ok
    (CallFunction|PickRandomAttachPoint)
    (CallFunction|RandomizeEnemies)
    (CallFunction|RandomizeShower)))

(event Collision|EventActorBeginOverlap
  (params (OtherActor :type Actor%20Object%20Reference)))

(event EventTick
  (params (DeltaSeconds :type Float%20%28single-precision%29)))

(event EventDestroyed
  (Development|PrintString "bye"))

(fn ConstructionScript
  (CallFunction|RandomizeEnvironment))

(fn PickRandomAttachPoint
  (LocalVariables|SetIndex (Math|Random|RandomIntegerinRange 0 2))
  (if (<= (Variables|Default|GetTilesLeft) 0)
    (Game|SpawnActorfromClass "/Game/Interactive/BP_ToiletPortal.BP_ToiletPortal_C" (Transformation|GetWorldTransform (Variables|Default|GetToiletPlace)) "Undefined" 0 0)
    (return)
    (else
      (bind _output_get (LocalVariables|SetPoints (Utilities|Array|MakeArray (Variables|Default|GetRightGate) (Variables|Default|GetLeftGate) (Variables|Default|GetFwdGate))))
      (CallFunction|SpawnatPoint (Utilities|Array|Get(acopy) _output_get (LocalVariables|GetIndex)))
      (bind _asbp_gate (Utilities|Casting|CastToBP_Gate (Variables|/Script/Engine.ChildActorComponent|GetChildActor (Utilities|Array|Get(acopy) _output_get (LocalVariables|GetIndex)))))
      (Default|Open _asbp_gate))))

(fn SpawnatPoint
  (params (component :type Scene%20Component%20Object%20Reference))
  (Game|SpawnActorfromClass :Class "BP_MapTile_C" :SpawnTransform (Math|Transform|MakeTransform (Transformation|GetWorldLocation component) (.rotation (Transformation|GetWorldTransform component)) (Math|Vector|MakeVector 0.5 0.5 0.5)) :CollisionHandlingOverride "Undefined" :TilesLeft (- (Variables|Default|GetTilesLeft) 1) :Instigator 0))

(fn OpenGate
  (params (OtherTile :type BP%20Map%20Tile%20Object%20Reference))
  (bind _dist (CallFunction|DistanceBetween (Variables|Default|GetRightGate) OtherTile))
  (LocalVariables|SetRightDist _dist)
  (bind _dist_2 (CallFunction|DistanceBetween (Variables|Default|GetLeftGate) OtherTile))
  (LocalVariables|SetLeftDist _dist_2)
  (bind _dist_3 (CallFunction|DistanceBetween (Variables|Default|GetFwdGate) OtherTile))
  (LocalVariables|SetFwdDist _dist_3)
  (if (Math|Float|NearlyEqual(Float) (Math|Float|Min(Float) (LocalVariables|GetLeftDist) (LocalVariables|GetRightDist) (LocalVariables|GetFwdDist)) (LocalVariables|GetLeftDist) 1e-06)
    (CallFunction|OpenSpecificGate (Variables|Default|GetLeftGate))
    (elif (Math|Float|NearlyEqual(Float) (Math|Float|Min(Float) (LocalVariables|GetLeftDist) (LocalVariables|GetRightDist) (LocalVariables|GetFwdDist)) (LocalVariables|GetRightDist) 1e-06)
      (CallFunction|OpenSpecificGate (Variables|Default|GetRightGate))
      (else
        (CallFunction|OpenSpecificGate (Variables|Default|GetFwdGate))))))

(fn DistanceBetween
  (params (gate :type Scene%20Component%20Object%20Reference) (tile :type BP%20Map%20Tile%20Object%20Reference))
  (return (Math|Vector|VectorLength (- (.location (Transformation|GetWorldTransform gate)) (Transformation|GetActorLocation tile)))))

(fn OpenSpecificGate
  (params (Gate :type Child%20Actor%20Component%20Object%20Reference))
  (Default|Open (.AsBP%20Gate (Utilities|Casting|CastToBP_Gate (Variables|/Script/Engine.ChildActorComponent|GetChildActor Gate)))))

(fn RandomizeEnvironment
  (for _array_element (Utilities|Array|MakeArray (Variables|Default|Getsink1) (Variables|Default|Getplant1) (Variables|Default|Gettoilet1) (Variables|Default|Gettoilet0) (Variables|Default|Getsink0) (Variables|Default|Getplant0) (Variables|Default|Getplant2) (Variables|Default|Getsink2) (Variables|Default|Getsink3) (Variables|Default|Getsink4) (Variables|Default|Gettoilet2))
    (if (<= (Math|Random|RandomFloat) 0.2)
      (Rendering|Components|Sprite|SetSprite _array_element 0))))

(fn RandomizeEnemies
  (for _array_element (Utilities|Array|MakeArray (Variables|Default|GetspawnPoint1) (Variables|Default|GetspawnPoint2) (Variables|Default|GetspawnPoint3) (Variables|Default|GetspawnPoint0))
    (if (not (Math|Random|RandomBool))
      (Game|SpawnActorfromClass (Utilities|Array|Get(acopy) (Variables|Default|GetEnemy%20Classess) (Math|Random|RandomInteger 2)) (Transformation|GetWorldTransform _array_element) "Undefined" 0 0))))

(fn RandomizeShower
  (if (not (>= (Math|Random|RandomFloat) 0.75))
    (Components|DestroyComponent (Variables|Default|GetShower))))