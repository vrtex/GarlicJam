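; BP_MazeGenerator is a maze generator actor that calls GenerateMaze on BeginPlay, returns to its starting point and prints the Maze length.
; The construction script caches the actor's location as StartingPoint, the origin of the grid.
; AddTile teleports the actor itself to an X/Y cell spaced at twice TileSize, without spawning anything in this graph.
; Open calls SetStaticMesh on StaticMesh1 with no mesh specified.
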(event EventBeginPlay
  (Class|Maze|GenerateMaze)
  (Transformation|SetActorLocation (Variables|Default|GetStartingPoint) false false)
  (Development|PrintString (Utilities|String|ToString(Integer) (Utilities|Array|Length (Variables|Default|Getmaze)))))

(event Collision|EventActorBeginOverlap
  (params (OtherActor :type Actor%20Object%20Reference)))

(event EventTick
  (params (DeltaSeconds :type Float%20%28single-precision%29)))

(event EventAddTile
  (params (x :type Integer) (y :type Integer) (leftWall :type Boolean) (rightWall :type Boolean) (upWall :type Boolean) (downWall :type Boolean))
  (bind _startingpoint (Variables|Default|GetStartingPoint))
  (bind _tilesize (Variables|Default|GetTileSize))
  (bind _returnvalue (* _tilesize 2.0))
  (Transformation|SetActorLocation (Math|Vector|MakeVector (+ (.x _startingpoint) (* x _returnvalue)) (+ (.y _startingpoint) (* y _returnvalue)) (.z _startingpoint)) false true))

(fn ConstructionScript
  (Variables|Default|SetStartingPoint (Transformation|GetActorLocation)))

(fn Open
  (Components|StaticMesh|SetStaticMesh (Variables|Default|GetStaticMesh1) 0))