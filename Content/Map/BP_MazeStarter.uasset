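; BP_MazeStarter is the first tile of a maze, the point from which the map starts.
; On BeginPlay it adds itself to BP_GameMode's tiles, sets itself as FirstTile, then calls PickRandomAttachPoint, which is defined outside this graph.
; Its reset event calls PickRandomAttachPoint again without repeating the registration.
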(event Custom|reset
  (CallFunction|PickRandomAttachPoint))

(event EventBeginPlay
  (bind _self self)
  (bind _asbp_game_mode (Utilities|Casting|CastToBP_GameMode (Game|GetGameMode)))
  (Default|AddTile _asbp_game_mode _self)
  (Variables|/Game/Misc/BP_GameMode.BP_GameMode_C|SetFirstTile _asbp_game_mode _self)
  (CallFunction|PickRandomAttachPoint))

(event Collision|EventActorBeginOverlap
  (params (OtherActor :type Actor%20Object%20Reference))
  (|CallParentFunction OtherActor) ; This node is disabled and will not be called.\nDrag off pins to build functionality.
)

(event EventTick
  (params (DeltaSeconds :type Float%20%28single-precision%29))
  (|CallParentFunction DeltaSeconds) ; This node is disabled and will not be called.\nDrag off pins to build functionality.
)

(fn ConstructionScript
  (|CallParentFunction))