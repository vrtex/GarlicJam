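; Player hero Blueprint using Paper2D flipbooks, where lost health shows as dirt on the character and in a dirt bar widget.
; A looping timer picks idle, walking or attack flipbooks by state and dirt level.
; Attacks spawn a damage blob along the last movement direction, Clean restores health, and zero health has the controller end the game.
; An active portal shows a prompt and enables teleporting.
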(event Custom|UpdateSprite
  (bind _spritescalefactor (Variables|Default|GetSpriteScaleFactor))
  (Sprite|SetFlipbook (Variables|Default|GetPaperFlipbook) (CallFunction|GetCurrentSprite))
  (Transformation|SetRelativeScale3D (Variables|Default|GetPaperFlipbook) (Math|Vector|MakeVector (select (and (< (.y (Transformation|GetVelocity)) 0.0) (== (Class|PaperFlipbookComponent|GetFlipbook (Variables|Default|GetPaperFlipbook)) (Variables|Default|GetWalkingAnimation))) (* _spritescalefactor 1.0) _spritescalefactor) _spritescalefactor _spritescalefactor)))

(event Custom|Attack
  (bind _returnvalue (Transformation|GetActorTransform))
  (Game|SpawnActorfromClass "/Game/MainHero/DamageBlob/BP_DamageBlob.BP_DamageBlob_C" (Math|Transform|MakeTransform (+ (.location _returnvalue) (* (Variables|Default|GetlastMovementDirection) 5e+01)) (.rotation _returnvalue) (.scale _returnvalue)) "Undefined" 0 0)
  (Components|Timeline|PlayfromStart (Variables|Default|GetPaperFlipbook))
  (Variables|Default|SetAttacking true)
  (Utilities|Time|SetTimerbyEvent (delegate Custom|reset%20attack) 0.5))

(event Custom|reset%20attack
  (Variables|Default|SetAttacking false))

(event EventBeginPlay
  (Utilities|Time|SetTimerbyEvent (delegate Custom|UpdateSprite) 0.1 true)
  (bind _returnvalue (UserInterface|CreateWidget "/Game/MainHero/UI/UI_DirtBar.UI_DirtBar_C" 0 self))
  (UserInterface|Viewport|AddtoViewport _returnvalue 0)
  (bind _returnvalue_2 (UserInterface|CreateWidget "/Game/MainHero/UI/UI_TeleportText.UI_TeleportText_C"))
  (Variables|Default|SetTeleportText _returnvalue_2))

(event Collision|EventActorBeginOverlap
  (params (OtherActor :type Actor%20Object%20Reference)))

(event EventTick
  (params (DeltaSeconds :type Float%20%28single-precision%29)))

(event Game|Damage|EventAnyDamage
  (params (Damage :type Float%20%28single-precision%29) (DamageType :type Damage%20Type%20Object%20Reference) (InstigatedBy :type Controller%20Object%20Reference) (DamageCauser :type Actor%20Object%20Reference))
  (Variables|Default|SetHealth (Math|Float|Clamp(Float) (- (Variables|Default|GetHealth) Damage) 0.0 (Variables|Default|GetMaxHelth)))
  (if (<= (Variables|Default|GetHealth) 0.0)
    (Audio|Components|Audio|Stop (Variables|Default|GetPaperFlipbook))
    (bind _asbp_main_hero_controller (Utilities|Casting|CastToBP_MainHeroController (Pawn|GetController)))
    (Default|EndGame _asbp_main_hero_controller)))

(fn ConstructionScript)

(fn GetCurrentSprite
  (bind _dirtlevel (CallFunction|GetDirtLevel))
  (if (Variables|Default|GetAttacking)
    (return (Utilities|Array|Get(acopy) (Variables|Default|GetAttackAnimations) (CallFunction|GetDirtLevel)))
    (else
      (return (select (> 0.01 (Math|Vector|VectorLength (Transformation|GetVelocity))) (Utilities|Array|Get(acopy) (Variables|Default|GetIdleAnimations) _dirtlevel) (Utilities|Array|Get(acopy) (Variables|Default|GetWalkingAnimations) _dirtlevel))))))

(fn GetDirtPercentage
  (return (- 1.0 (CallFunction|GetHealthPercentage))))

(fn GetHealthPercentage
  (if (Math|Float|NearlyEqual(Float) (Variables|Default|GetHealth) 0.0 1e-06)
    (return 0.0)
    (else
      (return (/ (Variables|Default|GetHealth) (Variables|Default|GetMaxHelth))))))

(fn GetDirtLevel
  (return (/ (Math|Float|Round (* (CallFunction|GetDirtPercentage) 1e+02)) 15)))

(fn Clean
  (params (Amount :type Float%20%28single-precision%29))
  (Variables|Default|SetHealth (Math|Float|Clamp(Float) (+ (Variables|Default|GetHealth) Amount) 0.0 (Variables|Default|GetMaxHelth))))

(fn SetActivePortal
  (params (Portal :type BP%20Toilet%20Portal%20Object%20Reference))
  (bind _teleporttext (Variables|Default|GetTeleportText))
  (bind _output_get (Variables|Default|SetActivePortal Portal))
  (bind _output_get_2 (Variables|Default|SetCanTeleport (Utilities|IsValid _output_get)))
  (if _output_get_2
    (UserInterface|Viewport|AddtoViewport _teleporttext 0)
    (else
      (Widget|RemovefromParent _teleporttext))))

(fn UseTeleport
  (if (Variables|Default|GetCanTeleport)
    (bind _teleportdestination (Default|Use (Variables|Default|GetActivePortal)))
    (Transformation|SetActorTransform _teleportdestination)
    (CallFunction|SetActivePortal)
    (else
      (return))))