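; BP_Shower is an interactive shower that cleans BP_MainHero while the hero stands in its box trigger, until its water runs out.
; Entering shifts the sprite doors aside, makes them translucent and starts particles plus a looping timer; leaving reverses this.
; TickCleaning cleans the stored hero and drains WaterLeft on each call, stopping the timer and particles once the water is empty.
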(event OnComponentBeginOverlap(Box)
  (params (OverlappedComponent :type Primitive%20Component%20Object%20Reference) (OtherActor :type Actor%20Object%20Reference) (OtherComp :type Primitive%20Component%20Object%20Reference) (OtherBodyIndex :type Integer) (bFromSweep :type Boolean) (SweepResult :type Hit%20Result%20Structure%20%28by%20ref%29))
  (bind _asbp_main_hero (Utilities|Casting|CastToBP_MainHero OtherActor))
  (Variables|Default|SetCleanedHero _asbp_main_hero)
  (Transformation|AddRelativeLocation (Variables|Default|GetDoors) "0,30.000000, 0" false false)
  (Sprite|SetSpriteColor (Variables|Default|GetDoors) "(R=1.000000,G=1.000000,B=1.000000,A=0.200000)")
  (CallFunction|StartCleaning))

(event OnComponentEndOverlap(Box)
  (params (OverlappedComponent :type Primitive%20Component%20Object%20Reference) (OtherActor :type Actor%20Object%20Reference) (OtherComp :type Primitive%20Component%20Object%20Reference) (OtherBodyIndex :type Integer))
  (Utilities|Casting|CastToBP_MainHero OtherActor)
  (Variables|Default|SetCleanedHero 0)
  (Transformation|AddRelativeLocation (Variables|Default|GetDoors) "0,-30.000000, 0" false false)
  (Sprite|SetSpriteColor (Variables|Default|GetDoors) "(R=1.000000,G=1.000000,B=1.000000,A=1.000000)")
  (CallFunction|StopCleaning))

(event EventBeginPlay)

(event Collision|EventActorBeginOverlap
  (params (OtherActor :type Actor%20Object%20Reference)))

(event EventTick
  (params (DeltaSeconds :type Float%20%28single-precision%29)))

(fn ConstructionScript)

(fn StartCleaning
  (bind _returnvalue (Utilities|Time|SetTimerbyEvent (EventDispatchers|CreateEvent :!event TickCleaning) 0.1 true))
  (Variables|Default|SetHealTimer _returnvalue)
  (Components|Activation|Activate (Variables|Default|GetParticleSystem) false))

(fn StopCleaning
  (Utilities|Time|InvalidateTimerHandle (Variables|Default|GetHealTimer))
  (Components|Activation|Deactivate (Variables|Default|GetParticleSystem)))

(fn TickCleaning
  (bind _cleanedhero (Variables|Default|GetCleanedHero))
  (if (<= (Variables|Default|GetWaterLeft) 0.0)
    (CallFunction|StopCleaning)
    (else
      (Utilities|IsValid _cleanedhero
        (:Is%20Valid
          (Default|Clean _cleanedhero 1.0)
          (Variables|Default|SetWaterLeft (- (Variables|Default|GetWaterLeft) 1.0)))))))