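; BP_ToiletPortal is an interactive level portal that generates the next maze or the boss room for the hero.
; Its box overlap registers it as BP_MainHero's active portal and clears that on exit.
; Use increments the game mode's CurrentLevel, spawning BP_BossRoom at level 3 and BP_MazeStarter otherwise.
; The new area spawns at half scale above the portal, and Use returns its player spawn.
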(event OnComponentBeginOverlap(Box)
  (params (OverlappedComponent :type Primitive%20Component%20Object%20Reference) (OtherActor :type Actor%20Object%20Reference) (OtherComp :type Primitive%20Component%20Object%20Reference) (OtherBodyIndex :type Integer) (bFromSweep :type Boolean) (SweepResult :type Hit%20Result%20Structure%20%28by%20ref%29))
  (bind _asbp_main_hero (Utilities|Casting|CastToBP_MainHero OtherActor))
  (Default|SetActivePortal _asbp_main_hero self))

(event OnComponentEndOverlap(Box)
  (params (OverlappedComponent :type Primitive%20Component%20Object%20Reference) (OtherActor :type Actor%20Object%20Reference) (OtherComp :type Primitive%20Component%20Object%20Reference) (OtherBodyIndex :type Integer))
  (bind _asbp_main_hero (Utilities|Casting|CastToBP_MainHero OtherActor))
  (Default|SetActivePortal _asbp_main_hero))

(event EventBeginPlay)

(event Collision|EventActorBeginOverlap
  (params (OtherActor :type Actor%20Object%20Reference)))

(event EventTick
  (params (DeltaSeconds :type Float%20%28single-precision%29)))

(fn ConstructionScript)

(fn Use
  (bind _result (Math|Integer|IncrementInt (Variables|/Game/Misc/BP_GameMode.BP_GameMode_C|GetcurrentLevel (.AsBP%20Game%20Mode (Utilities|Casting|CastToBP_GameMode (Game|GetGameMode)))))
    (:%20%20
      (bind _output_get (LocalVariables|SetDestination (+ (Transformation|GetActorLocation) "0, 0,1000.000000")))
      (if (== _result 3)
        (bind _returnvalue (Game|SpawnActorfromClass "/Game/Map/BP_BossRoom.BP_BossRoom_C" (Math|Transform|MakeTransform _output_get "0, 0, 0" "0.500000,0.500000,0.500000") "Undefined" 0 0))
        (return (Default|GetPlayerSpawn _returnvalue))
        (else
          (bind _returnvalue_2 (Game|SpawnActorfromClass :Class "/Game/Map/BP_MazeStarter.BP_MazeStarter_C" :SpawnTransform (Math|Transform|MakeTransform _output_get "0, 0, 0" "0.500000,0.500000,0.500000") :CollisionHandlingOverride "Undefined" :Instigator 0))
          (return (Default|GetPlayerSpawn _returnvalue_2)))))))