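; Game mode that links placed tiles by opening gates between neighbours.
; AddTile compares the new tile against the Tiles array and, for each within 300 units, calls OpenTiles to open gates both ways.
; AddTile always returns true and does not itself append to Tiles.
; ResetTiles only prints a notice, as its logic to destroy tiles and reset FirstTile is disconnected.
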(event EventBeginPlay)

(event EventTick
  (params (DeltaSeconds :type Float%20%28single-precision%29)))

(fn ConstructionScript)

(fn AddTile
  (params (TileToAdd :type BP%20Map%20Tile%20Object%20Reference))
  (for _array_element (Variables|Default|GetTiles)
    (if (<= (Math|Vector|VectorLength (- (Transformation|GetActorLocation TileToAdd) (Transformation|GetActorLocation _array_element))) 3e+02)
      (CallFunction|OpenTiles TileToAdd _array_element)))
  (return true))

(fn ResetTiles
  (Development|PrintString "reset turned off, reconnect pin"))

(fn OpenTiles
  (params (A :type BP%20Map%20Tile%20Object%20Reference) (B :type BP%20Map%20Tile%20Object%20Reference))
  (Default|OpenGate A B)
  (Default|OpenGate B A))