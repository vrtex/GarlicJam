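; Boss enemy with a flipbook sprite and high health whose defeat wins the game.
; A looping timer spawns a random minion class at a short offset in a random direction.
; Each spawn halts movement while the Pop timeline scales the sprite, then restores walk speed when it finishes.
; Damage runs through the parent class, then zero health calls WinGame on the player's BP_MainHeroController.
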(event Custom|Spwan%20Minion
  (bind _minion_classes (Variables|Default|GetMinion%20Classes))
  (Game|SpawnActorfromClass (Utilities|Array|Get(acopy) _minion_classes (Math|Random|RandomInteger (Utilities|Array|Length _minion_classes))) (Math|Transform|MakeTransform (+ (Transformation|GetActorLocation) (* (Math|Rotator|GetRotationXVector (Math|Random|RandomRotator false)) 1e+02))) "AdjustIfPossibleButAlwaysSpawn" 0 0)
  (Variables|/Script/Engine.CharacterMovementComponent|SetMaxWalkSpeed (Variables|Character|GetCharacterMovement) 0.0)
  (bind _newtrack_0 (Timeline|Pop PlayFromStart)
    (:Update
      (Transformation|SetRelativeScale3D (Variables|Default|GetPaperFlipbook) (Math|Vector|MakeVector _newtrack_0 _newtrack_0 _newtrack_0)))
    (:Finished
      (Variables|/Script/Engine.CharacterMovementComponent|SetMaxWalkSpeed (Variables|Character|GetCharacterMovement) 1.5e+02))))

(event EventBeginPlay
  (bind _output_get (Variables|Default|SetMaxHealth 666.0))
  (Variables|Default|SetHealth _output_get)
  (Utilities|Time|SetTimerbyEvent (delegate Custom|Spwan%20Minion) 5.0 true))

(event Collision|EventActorBeginOverlap
  (params (OtherActor :type Actor%20Object%20Reference))
  (|CallParentFunction OtherActor) ; This node is disabled and will not be called.\nDrag off pins to build functionality.
)

(event EventTick
  (params (DeltaSeconds :type Float%20%28single-precision%29))
  (|CallParentFunction DeltaSeconds) ; This node is disabled and will not be called.\nDrag off pins to build functionality.
)

(event Game|Damage|EventAnyDamage
  (params (Damage :type Float%20%28single-precision%29) (DamageType :type Damage%20Type%20Object%20Reference) (InstigatedBy :type Controller%20Object%20Reference) (DamageCauser :type Actor%20Object%20Reference))
  (|CallParentFunction Damage DamageType InstigatedBy DamageCauser)
  (if (<= (Variables|Default|GetHealth) 0.0)
    (Default|WinGame (.AsBP%20Main%20Hero%20Controller (Utilities|Casting|CastToBP_MainHeroController (Game|GetPlayerController 0))))))

(fn ConstructionScript
  (|CallParentFunction))