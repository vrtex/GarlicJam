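; BP_BasicPoop is a Paper2D enemy character that can attack the hero and die, leaving a BP_DeadPoop behind.
; A looping timer calls CheckForTarget and applies a small upward force.
; AttackHero deals damage with a brief Farting effect, while taking damage lowers Health, blinks the flipbook red, then checks for death.
; Sphere overlap events are empty, leaving the blackboard TargetHero logic disconnected.
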(event OnComponentBeginOverlap(Sphere)
  (params (OverlappedComponent :type Primitive%20Component%20Object%20Reference) (OtherActor :type Actor%20Object%20Reference) (OtherComp :type Primitive%20Component%20Object%20Reference) (OtherBodyIndex :type Integer) (bFromSweep :type Boolean) (SweepResult :type Hit%20Result%20Structure%20%28by%20ref%29)))

(event OnComponentEndOverlap(Sphere)
  (params (OverlappedComponent :type Primitive%20Component%20Object%20Reference) (OtherActor :type Actor%20Object%20Reference) (OtherComp :type Primitive%20Component%20Object%20Reference) (OtherBodyIndex :type Integer)))

(event Custom|CustomEvent_0
  (Class|BasicPoop|CheckforTarget)
  (Physics|AddForce (Variables|Character|GetCharacterMovement) "0, 0,10.000000"))

(event Custom|AttackHero
  (params (Hero :type BP%20Main%20Hero%20Object%20Reference))
  (Game|Damage|ApplyDamage Hero 1e+01 (AI|GetAIController 0) 0)
  (Components|Activation|Activate (Variables|Default|GetFarting) false)
  (Utilities|Time|SetTimerbyEvent (delegate Custom|fart%20reset) 0.1))

(event Custom|fart%20reset
  (Components|Activation|Deactivate (Variables|Default|GetFarting)))

(event EventBeginPlay
  (Utilities|Time|SetTimerbyEvent (delegate Custom|CustomEvent_0) 0.1 true))

(event Collision|EventActorBeginOverlap
  (params (OtherActor :type Actor%20Object%20Reference)))

(event EventTick
  (params (DeltaSeconds :type Float%20%28single-precision%29)))

(event Game|Damage|EventAnyDamage
  (params (Damage :type Float%20%28single-precision%29) (DamageType :type Damage%20Type%20Object%20Reference) (InstigatedBy :type Controller%20Object%20Reference) (DamageCauser :type Actor%20Object%20Reference))
  (bind _output_get (Variables|Default|SetHealth (- (Variables|Default|GetHealth) Damage)))
  (bind _alpha (Timeline|Blink PlayFromStart)
    (:Update
      (Sprite|SetSpriteColor (Variables|Default|GetPaperFlipbook) (Math|Color|Lerp(LinearColor) "(R=1.000000,G=1.000000,B=1.000000,A=1.000000)" "(R=0.467784,G=0.004777,B=0.000000,A=1.000000)" _alpha)))
    (:Finished
      (if (< _output_get 0.0)
        (Game|SpawnActorfromClass "/Game/Enemies/BP_DeadPoop.BP_DeadPoop_C" (Transformation|GetActorTransform) "Undefined" 0 (Variables|/Script/Engine.SceneComponent|GetRelativeScale3D (Variables|Default|GetPaperFlipbook)) (Variables|Default|GetDeadSprite) 0)
        (Actor|DestroyActor)))))

(fn ConstructionScript)