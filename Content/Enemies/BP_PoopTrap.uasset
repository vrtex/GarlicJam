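; BP_PoopTrap is a short-lived enemy hazard that damages BP_MainHero while it overlaps the trap's sprites.
; The construction script scatters three sprites at random X/Y offsets around the actor origin.
; A looping half-second timer applies DamageValue per overlapped sprite, so overlapping several sprites stacks damage.
; A second timer destroys the actor after three seconds.
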(event Custom|Try%20Apply%20Damage
  (for _array_element (Collision|GetOverlappingActors (Variables|Default|GetSprite) "/Game/MainHero/BP_MainHero.BP_MainHero_C" :!class /Script/Engine.PrimitiveComponent)
    (Game|Damage|ApplyDamage (.AsBP%20Main%20Hero (Utilities|Casting|CastToBP_MainHero _array_element)) (Variables|Default|GetDamageValue) 0 0))
  (for _array_element_2 (Collision|GetOverlappingActors (Variables|Default|GetSprite1) "/Game/MainHero/BP_MainHero.BP_MainHero_C" :!class /Script/Engine.PrimitiveComponent)
    (Game|Damage|ApplyDamage (.AsBP%20Main%20Hero (Utilities|Casting|CastToBP_MainHero _array_element_2)) (Variables|Default|GetDamageValue) 0 0))
  (for _array_element_3 (Collision|GetOverlappingActors (Variables|Default|GetSprite2) "/Game/MainHero/BP_MainHero.BP_MainHero_C" :!class /Script/Engine.PrimitiveComponent)
    (Game|Damage|ApplyDamage (.AsBP%20Main%20Hero (Utilities|Casting|CastToBP_MainHero _array_element_3)) (Variables|Default|GetDamageValue) 0 0)))

(event Custom|AutoDestruct
  (Actor|DestroyActor))

(event EventBeginPlay
  (Utilities|Time|SetTimerbyEvent (delegate Custom|Try%20Apply%20Damage) 0.5 true)
  (Utilities|Time|SetTimerbyEvent (delegate Custom|AutoDestruct) 3.0))

(event Collision|EventActorBeginOverlap
  (params (OtherActor :type Actor%20Object%20Reference)))

(event EventTick
  (params (DeltaSeconds :type Float%20%28single-precision%29)))

(fn ConstructionScript
  (bind _returnvalue (Math|Vector|MakeVector 5.0 5.0 0.0))
  (bind _returnvalue_2 (Math|Vector|MakeVector 0.0 0.0 0.0))
  (bind _returnvalue_3 (Math|Random|RandomPointinBoundingBox _returnvalue_2 _returnvalue))
  (bind _returnvalue_4 (* _returnvalue_3 1e+01))
  (Transformation|SetRelativeLocation (Variables|Default|GetSprite) _returnvalue_4 false false)
  (Transformation|SetRelativeLocation (Variables|Default|GetSprite1) _returnvalue_4 false false)
  (Transformation|SetRelativeLocation (Variables|Default|GetSprite2) _returnvalue_4 false false))